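; Tutorial HUD that draws a multiplayer main menu and a lobby screen on the canvas, chosen by state flags.
; DrawButton renders textured, centered-label buttons with hit boxes, whose clicks set pressed textures and releases issue console commands.
; Host, Join and Quit handle sessions, while a server-only Start triggers ServerTravel to the game level.
; Digit, period and delete key events edit the IP string shown for joining.
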(event `self.ReceiveBeginPlay`
  (`KismetSystemLibrary.PrintString` "HUD drawn"))

(event `self.ReceiveDrawHUD`
  (params (SizeX :type Integer) (SizeY :type Integer))
  (bind _buttontexture (`self.ButtonTexture`))
  (bind (_x _y) (`KismetMathLibrary.BreakVector2D` (`self.ScreenDimensions`)))
  (bind (_x_2 _y_2) (`KismetMathLibrary.BreakVector2D` (`self.ScreenDimensions`)))
  (set `self.ButtonSize` (`KismetMathLibrary.MakeVector2D` (`KismetMathLibrary.Conv_IntToDouble` (`Texture2D.Blueprint_GetSizeX` _buttontexture)) (`KismetMathLibrary.Conv_IntToDouble` (`Texture2D.Blueprint_GetSizeY` _buttontexture))))
  (set `self.ScreenDimensions` (`KismetMathLibrary.MakeVector2D` (`KismetMathLibrary.Conv_IntToDouble` SizeX) (`KismetMathLibrary.Conv_IntToDouble` SizeY)))
  (if (`self.MainMenuIsActive`)
    (`self.DrawMaterialSimple` "/Game/MenuTutorial/Misc/TutorialMenuMat.TutorialMenuMat" 0.0 0.0 _x _y)
    (`self.DrawRect` (`self.TextBackgroundColor`) 700.0 700.0 400.0 50.0)
    (`self.DrawText` (`self.ipString`) (`self.TextColor`) 700.0 700.0 "/Game/MenuTutorial/Misc/TutorialFont.TutorialFont" 2.0)
    (`self.DrawButton` (`KismetMathLibrary.MakeVector2D` 10.0 400.0) (`self.ButtonSize`) "Host" (select `bool` (`self.HostButtonPressed`) :`false` (`self.ButtonTexture`) :`true` (`self.ButtonTexturePressed`)) (`self.TextColor`))
    (`self.DrawButton` (`KismetMathLibrary.MakeVector2D` 10.0 600.0) (`self.ButtonSize`) "Join" (select `bool` (`self.JoinButtonPressed`) :`false` (`self.ButtonTexture`) :`true` (`self.ButtonTexturePressed`)) (`self.TextColor`))
    (`self.DrawButton` (`KismetMathLibrary.MakeVector2D` 10.0 800.0) (`self.ButtonSize`) "Quit" (select `bool` (`self.QuitButtonPressed`) :`false` (`self.ButtonTexture`) :`true` (`self.ButtonTexturePressed`)) (`self.TextColor`))
    (elif (`self.LobbyIsActive`)
      (`self.DrawMaterialSimple` "/Game/MenuTutorial/Misc/TutorialLobbyMat.TutorialLobbyMat" 0.0 0.0 _x_2 _y_2)
      (if (`KismetSystemLibrary.IsServer`)
        (`self.DrawButton` (`KismetMathLibrary.MakeVector2D` 10.0 400.0) (`self.ButtonSize`) "Start" (select `bool` (`self.StartButtonPressed`) :`false` (`self.ButtonTexture`) :`true` (`self.ButtonTexturePressed`)) (`self.TextColor`)))
      (`self.DrawButton` (`KismetMathLibrary.MakeVector2D` 10.0 600.0) (`self.ButtonSize`) "Quit" (select `bool` (`self.QuitButtonPressed`) :`false` (`self.ButtonTexture`) :`true` (`self.ButtonTexturePressed`)) (`self.TextColor`)))))

(event `self.ReceiveHitBoxClick`
  (params (BoxName :type Name))
  (switch `name` BoxName
    (:`Host`
      (set `self.HostButtonPressed` true))
    (:`Join`
      (set `self.JoinButtonPressed` true))
    (:`Quit`
      (set `self.QuitButtonPressed` true))
    (:`Start`
      (set `self.StartButtonPressed` true))))

(event `Key|NumPadOne`
  (params (Key :type "Key Structure" :default "AnyKey"))
  (:`Pressed`
    (`self.BuildHostString` "1" :!label _label)))

(event `Key|One`
  (params (Key :type "Key Structure" :default "AnyKey"))
  (:`Pressed`
    (goto _label)))

(event `Key|NumPadTwo`
  (params (Key :type "Key Structure" :default "AnyKey"))
  (:`Pressed`
    (`self.BuildHostString` "2" :!label _label_2)))

(event `Key|Two`
  (params (Key :type "Key Structure" :default "AnyKey"))
  (:`Pressed`
    (goto _label_2)))

(event `Key|NumPadThree`
  (params (Key :type "Key Structure" :default "AnyKey"))
  (:`Pressed`
    (`self.BuildHostString` "3" :!label _label_3)))

(event `Key|Three`
  (params (Key :type "Key Structure" :default "AnyKey"))
  (:`Pressed`
    (goto _label_3)))

(event `self.ReceiveHitBoxRelease`
  (params (BoxName :type Name))
  (switch `name` BoxName
    (:`Host`
      (`KismetSystemLibrary.ExecuteConsoleCommand` (`KismetStringLibrary.Concat_StrStr` "Open " "Lobby?Listen")))
    (:`Join`
      (`KismetSystemLibrary.ExecuteConsoleCommand` (`KismetStringLibrary.Concat_StrStr` "Open " (`self.ipString`))))
    (:`Quit`
      (`KismetSystemLibrary.ExecuteConsoleCommand` "Exit"))
    (:`Start`
      (set `self.LobbyIsActive` false)
      (set `self.MainMenuIsActive` false)
      (`KismetSystemLibrary.ExecuteConsoleCommand` (`KismetStringLibrary.Concat_StrStr` "ServerTravel " (`self.GameLevelName`))))))

(event `Key|NumPadFour`
  (params (Key :type "Key Structure" :default "AnyKey"))
  (:`Pressed`
    (`self.BuildHostString` "4" :!label _label_4)))

(event `Key|Four`
  (params (Key :type "Key Structure" :default "AnyKey"))
  (:`Pressed`
    (goto _label_4)))

(event `Key|NumPadFive`
  (params (Key :type "Key Structure" :default "AnyKey"))
  (:`Pressed`
    (`self.BuildHostString` "5" :!label _label_5)))

(event `Key|Five`
  (params (Key :type "Key Structure" :default "AnyKey"))
  (:`Pressed`
    (goto _label_5)))

(event `Key|NumPadSix`
  (params (Key :type "Key Structure" :default "AnyKey"))
  (:`Pressed`
    (`self.BuildHostString` "6" :!label _label_6)))

(event `Key|Six`
  (params (Key :type "Key Structure" :default "AnyKey"))
  (:`Pressed`
    (goto _label_6)))

(event `Key|LeftMouseButton`
  (params (Key :type "Key Structure" :default "AnyKey"))
  (:`Released`
    (set `self.HostButtonPressed` false)
    (set `self.JoinButtonPressed` false)
    (set `self.QuitButtonPressed` false)
    (set `self.StartButtonPressed` false)))

(event `Key|NumPadSeven`
  (params (Key :type "Key Structure" :default "AnyKey"))
  (:`Pressed`
    (`self.BuildHostString` "7" :!label _label_7)))

(event `Key|Seven`
  (params (Key :type "Key Structure" :default "AnyKey"))
  (:`Pressed`
    (goto _label_7)))

(event `Key|NumPadEight`
  (params (Key :type "Key Structure" :default "AnyKey"))
  (:`Pressed`
    (`self.BuildHostString` "8" :!label _label_8)))

(event `Key|Eight`
  (params (Key :type "Key Structure" :default "AnyKey"))
  (:`Pressed`
    (goto _label_8)))

(event `Key|NumPadNine`
  (params (Key :type "Key Structure" :default "AnyKey"))
  (:`Pressed`
    (`self.BuildHostString` "9" :!label _label_9)))

(event `Key|Nine`
  (params (Key :type "Key Structure" :default "AnyKey"))
  (:`Pressed`
    (goto _label_9)))

(event `Key|NumPadZero`
  (params (Key :type "Key Structure" :default "AnyKey"))
  (:`Pressed`
    (`self.BuildHostString` "0" :!label _label_10)))

(event `Key|Zero`
  (params (Key :type "Key Structure" :default "AnyKey"))
  (:`Pressed`
    (goto _label_10)))

(event `Key|Decimal`
  (params (Key :type "Key Structure" :default "AnyKey"))
  (:`Pressed`
    (`self.BuildHostString` "." :!label _label_11)))

(event `Key|Period`
  (params (Key :type "Key Structure" :default "AnyKey"))
  (:`Pressed`
    (goto _label_11)))

(event `Key|Q`
  (params (Key :type "Key Structure" :default "AnyKey")))

(event `Key|BackSpace`
  (params (Key :type "Key Structure" :default "AnyKey"))
  (:`Pressed`
    (`self.DeleteStringCharacter` :!label _label_12)))

(event `Key|Delete`
  (params (Key :type "Key Structure" :default "AnyKey"))
  (:`Pressed`
    (goto _label_12)))

(fn `BuildHostString`
  (params (KeyInput :type String))
  (set `self.ipString` (`KismetStringLibrary.Concat_StrStr` (`self.ipString`) KeyInput)))

(fn `DeleteStringCharacter`
  (bind _ipstring (`self.ipString`))
  (set `self.ipString` (`KismetStringLibrary.GetSubstring` _ipstring 0 (- (`KismetStringLibrary.Len` _ipstring) 1))))

(fn `DrawButton`
  (params (ButtonScreenLocation :type "Vector2D Structure") (ButtonSize :type "Vector2D Structure") (ButtonText :type String) (Texture :type "Texture Object Reference") (TextColor :type "LinearColor Structure"))
  (bind (_x _y) (`KismetMathLibrary.BreakVector2D` ButtonScreenLocation))
  (bind (_outwidth _outheight) (`self.GetTextSize` ButtonText "/Game/MenuTutorial/Misc/TutorialFont.TutorialFont" 1.5))
  (bind (_x_2 _y_2) (`KismetMathLibrary.BreakVector2D` (- (+ (/ ButtonSize 2.0) ButtonScreenLocation) (/ (`KismetMathLibrary.MakeVector2D` _outwidth _outheight) 2.0))))
  (`self.DrawTextureSimple` Texture _x _y)
  (`self.DrawText` ButtonText TextColor _x_2 _y_2 "/Game/MenuTutorial/Misc/TutorialFont.TutorialFont" 1.5)
  (`self.AddHitBox` ButtonScreenLocation ButtonSize (`KismetStringLibrary.Conv_StringToName` ButtonText)))

(fn `UserConstructionScript`)