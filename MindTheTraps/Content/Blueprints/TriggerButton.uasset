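; Multiplayer pressure-button puzzle actor that sets Pressed when every active button, one per player up to four, is occupied.
; BeginPlay hides surplus cubes and disables their triggers using NumberOfPlayers, which InitVars counts from PlayerControllers but is not called here.
; Player-tagged overlaps raise per-button counters, swap materials and recheck completion.
; End overlaps decrement without a tag check, clearing Pressed when a counter reaches zero; the door-sound branch is disconnected.
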(event `Init Vars`
  (bind _outactors (`GameplayStatics.GetAllActorsOfClass` "/Script/Engine.PlayerController"))
  (set `self.NumberOfPlayers` (`KismetArrayLibrary.Array_Length` _outactors)))

(event `self.ReceiveBeginPlay`
  (if (< (`self.NumberOfPlayers`) 4)
    (`SceneComponent.ToggleVisibility` (`self.Cube3`) false)
    (`PrimitiveComponent.SetCollisionEnabled` (`self.TriggerVol3`) "NoCollision")
    (if (< (`self.NumberOfPlayers`) 3)
      (`SceneComponent.ToggleVisibility` (`self.Cube2`) false)
      (`PrimitiveComponent.SetCollisionEnabled` (`self.TriggerVol2`) "NoCollision")
      (if (< (`self.NumberOfPlayers`) 2)
        (`SceneComponent.ToggleVisibility` (`self.Cube1`) false)
        (`PrimitiveComponent.SetCollisionEnabled` (`self.TriggerVol1`) "NoCollision")))))

(event `self.TriggerVol.OnComponentBeginOverlap`
  (params (OtherActor :type "Actor Object Reference") (OtherComp :type "PrimitiveComponent Object Reference") (OtherBodyIndex :type Integer) (bFromSweep :type Boolean) (SweepResult :type "HitResult Structure (by ref)"))
  (bind _1press (`self.1Press`))
  (bind _2press (`self.2Press`))
  (bind _3press (`self.3Press`))
  (if (`self.ActorHasTag` OtherActor "Player")
    (`/Engine/EditorBlueprintResources/StandardMacros.IncrementInt` (`self.Target1Counter`)
      (:`  `
        (set `self.1Press` true)
        (`PrimitiveComponent.SetMaterial` (`self.Cube`) 0 "/Game/Materials/ButtonActivated.ButtonActivated")
        (if (== (`self.NumberOfPlayers`) 4) :!label _label
          (if (and _1press _2press _3press (`self.4Press`))
            (set `self.Pressed` true))
          (elif (== (`self.NumberOfPlayers`) 3)
            (if (and _1press _2press _3press)
              (set `self.Pressed` true))
            (elif (== (`self.NumberOfPlayers`) 2)
              (if (and _1press _2press)
                (set `self.Pressed` true))
              (elif (== (`self.NumberOfPlayers`) 1)
                (if _1press
                  (set `self.Pressed` true))))))))))

(event `self.TriggerVol.OnComponentEndOverlap`
  (params (OtherActor :type "Actor Object Reference") (OtherComp :type "PrimitiveComponent Object Reference") (OtherBodyIndex :type Integer))
  (bind _target1counter (`self.Target1Counter`))
  (`/Engine/EditorBlueprintResources/StandardMacros.DecrementInt` _target1counter
    (:`  `
      (if (== _target1counter 0)
        (set `self.1Press` false)
        (`PrimitiveComponent.SetMaterial` (`self.Cube`) 0 "/Game/Materials/ButtonDeactivated.ButtonDeactivated")
        (set `self.Pressed` false :!label _label_2)))))

(event `self.TriggerVol1.OnComponentBeginOverlap`
  (params (OtherActor :type "Actor Object Reference") (OtherComp :type "PrimitiveComponent Object Reference") (OtherBodyIndex :type Integer) (bFromSweep :type Boolean) (SweepResult :type "HitResult Structure (by ref)"))
  (if (`self.ActorHasTag` OtherActor "Player")
    (`/Engine/EditorBlueprintResources/StandardMacros.IncrementInt` (`self.Target2Counter`)
      (:`  `
        (set `self.2Press` true)
        (`PrimitiveComponent.SetMaterial` (`self.Cube1`) 0 "/Game/Materials/ButtonActivated.ButtonActivated")
        (goto _label)))))

(event `self.TriggerVol1.OnComponentEndOverlap`
  (params (OtherActor :type "Actor Object Reference") (OtherComp :type "PrimitiveComponent Object Reference") (OtherBodyIndex :type Integer))
  (bind _target2counter (`self.Target2Counter`))
  (`/Engine/EditorBlueprintResources/StandardMacros.DecrementInt` _target2counter
    (:`  `
      (if (== _target2counter 0)
        (set `self.2Press` false)
        (`PrimitiveComponent.SetMaterial` (`self.Cube1`) 0 "/Game/Materials/ButtonDeactivated.ButtonDeactivated")
        (goto _label_2)))))

(event `self.TriggerVol2.OnComponentBeginOverlap`
  (params (OtherActor :type "Actor Object Reference") (OtherComp :type "PrimitiveComponent Object Reference") (OtherBodyIndex :type Integer) (bFromSweep :type Boolean) (SweepResult :type "HitResult Structure (by ref)"))
  (if (`self.ActorHasTag` OtherActor "Player")
    (`/Engine/EditorBlueprintResources/StandardMacros.IncrementInt` (`self.Target3Counter`)
      (:`  `
        (set `self.3Press` true)
        (`PrimitiveComponent.SetMaterial` (`self.Cube2`) 0 "/Game/Materials/ButtonActivated.ButtonActivated")
        (goto _label)))))

(event `self.TriggerVol2.OnComponentEndOverlap`
  (params (OtherActor :type "Actor Object Reference") (OtherComp :type "PrimitiveComponent Object Reference") (OtherBodyIndex :type Integer))
  (bind _target3counter (`self.Target3Counter`))
  (`/Engine/EditorBlueprintResources/StandardMacros.DecrementInt` _target3counter
    (:`  `
      (if (== _target3counter 0)
        (set `self.3Press` false)
        (`PrimitiveComponent.SetMaterial` (`self.Cube2`) 0 "/Game/Materials/ButtonDeactivated.ButtonDeactivated")
        (goto _label_2)))))

(event `self.TriggerVol3.OnComponentBeginOverlap`
  (params (OtherActor :type "Actor Object Reference") (OtherComp :type "PrimitiveComponent Object Reference") (OtherBodyIndex :type Integer) (bFromSweep :type Boolean) (SweepResult :type "HitResult Structure (by ref)"))
  (if (`self.ActorHasTag` OtherActor "Player")
    (`/Engine/EditorBlueprintResources/StandardMacros.IncrementInt` (`self.Target4Counter`)
      (:`  `
        (set `self.4Press` true)
        (`PrimitiveComponent.SetMaterial` (`self.Cube3`) 0 "/Game/Materials/ButtonActivated.ButtonActivated")
        (goto _label)))))

(event `self.TriggerVol3.OnComponentEndOverlap`
  (params (OtherActor :type "Actor Object Reference") (OtherComp :type "PrimitiveComponent Object Reference") (OtherBodyIndex :type Integer))
  (bind _target4counter (`self.Target4Counter`))
  (`/Engine/EditorBlueprintResources/StandardMacros.DecrementInt` _target4counter
    (:`  `
      (if (== _target4counter 0)
        (set `self.4Press` false)
        (`PrimitiveComponent.SetMaterial` (`self.Cube3`) 0 "/Game/Materials/ButtonDeactivated.ButtonDeactivated")
        (goto _label_2)))))

(fn `UserConstructionScript`)