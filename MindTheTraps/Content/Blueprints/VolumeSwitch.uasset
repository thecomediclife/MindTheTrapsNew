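; VolumeSwitch is a trigger volume switch that detects when all players are inside it at once.
; Begin and end overlaps of actors tagged Player raise and lower a counter.
; On entry, only the authority compares the counter to NumberOfPlayers and sets AllPlayersEntered on a match.
; The flag latches, as nothing in these graphs clears it when a player leaves.
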(event `self.Triggervol.OnComponentBeginOverlap`
  (params (OtherActor :type "Actor Object Reference") (OtherComp :type "PrimitiveComponent Object Reference") (OtherBodyIndex :type Integer) (bFromSweep :type Boolean) (SweepResult :type "HitResult Structure (by ref)"))
  (if (`self.ActorHasTag` OtherActor "Player")
    (`/Engine/EditorBlueprintResources/StandardMacros.IncrementInt` (`self.PlayerCounter`)
      (:`  `
        (`/Engine/EditorBlueprintResources/ActorMacros.Switch Has Authority`
          (:`Authority`
            (if (== (`self.PlayerCounter`) (`self.NumberOfPlayers`))
              (set `self.AllPlayersEntered` true))))))))

(event `self.Triggervol.OnComponentEndOverlap`
  (params (OtherActor :type "Actor Object Reference") (OtherComp :type "PrimitiveComponent Object Reference") (OtherBodyIndex :type Integer))
  (if (`self.ActorHasTag` OtherActor "Player")
    (`/Engine/EditorBlueprintResources/StandardMacros.DecrementInt` (`self.PlayerCounter`))))

(fn `UserConstructionScript`)