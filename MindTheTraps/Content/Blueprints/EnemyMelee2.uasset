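; Melee enemy that chases a tagged Player1 entering its sight sphere with the torch enabled, optionally returning to its start when sight is lost.
; While Activated, Tick interpolates location and rotation directly toward the target, without navigation.
; DamageCheck overlaps fire a radial impulse, then either hurt the player or, if TorchDisabled, cost the enemy health.
; DoOnce gates limit hits; the enemy flashes its material when hurt and explodes at zero health.
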(event `self.ReceiveBeginPlay`
  (set `self.OriginalPos` (`self.K2_GetActorLocation`)))

(event `self.Sphere.OnComponentEndOverlap`
  (params (OtherActor :type "Actor Object Reference") (OtherComp :type "PrimitiveComponent Object Reference") (OtherBodyIndex :type Integer))
  (if (== OtherActor (`self.Target`))
    (set `self.PlayerInSight` false)))

(event `self.Sphere.OnComponentBeginOverlap`
  (params (OtherActor :type "Actor Object Reference") (OtherComp :type "PrimitiveComponent Object Reference") (OtherBodyIndex :type Integer) (bFromSweep :type Boolean) (SweepResult :type "HitResult Structure (by ref)"))
  (if (`self.ActorHasTag` OtherActor "Player")
    (bind _asplayer_1 (cast `/Game/Characters/Player1` OtherActor))
    (if (not (`/Game/Characters/Player1.TorchDisabled` _asplayer_1))
      (set `self.Target` OtherActor)
      (set `self.PlayerInSight` true))))

(event `self.ReceiveTick`
  (params (DeltaSeconds :type "Float (single-precision)"))
  (bind _returnvalue (`self.K2_GetActorLocation`))
  (bind _returnvalue_2 (`self.K2_GetActorLocation`))
  (bind _originalpos (`self.OriginalPos`))
  (bind _returnvalue_3 (`KismetMathLibrary.MakeVector` (.x (`self.K2_GetActorLocation` (`self.Target`))) (.y (`self.K2_GetActorLocation` (`self.Target`))) (.z (`self.K2_GetActorLocation` (`self.Target`)))))
  (if (`self.Activated`)
    (if (`self.PlayerInSight`)
      (`self.K2_SetActorLocationAndRotation` (`KismetMathLibrary.VInterpTo` _returnvalue _returnvalue_3 DeltaSeconds (`self.MoveSpeed`)) (`KismetMathLibrary.RInterpTo` (`self.K2_GetActorRotation`) (`KismetMathLibrary.FindLookAtRotation` _returnvalue _returnvalue_3) DeltaSeconds (`self.TurnSpeed`)))
      (elif (`self.ReturnToOrigin`)
        (`self.K2_SetActorLocationAndRotation` (`KismetMathLibrary.VInterpTo` _returnvalue_2 _originalpos DeltaSeconds (`self.MoveSpeed`)) (`KismetMathLibrary.RInterpTo` (`self.K2_GetActorRotation`) (`KismetMathLibrary.FindLookAtRotation` _returnvalue_2 _originalpos) (`self.TurnSpeed`) DeltaSeconds))))))

(event `self.DamageCheck.OnComponentBeginOverlap`
  (params (OtherActor :type "Actor Object Reference") (OtherComp :type "PrimitiveComponent Object Reference") (OtherBodyIndex :type Integer) (bFromSweep :type Boolean) (SweepResult :type "HitResult Structure (by ref)"))
  (bind _skeletalmesh (`self.SkeletalMesh`))
  (if (`self.ActorHasTag` OtherActor "Player")
    (bind _asplayer_1 (cast `/Game/Characters/Player1` OtherActor))
    (if (`/Game/Characters/Player1.TorchDisabled` _asplayer_1)
      ;[1 1 1] get hit
      (`/Engine/EditorBlueprintResources/StandardMacros.DoOnce` false :!label _label
        (:`Completed`
          (`RadialForceComponent.FireImpulse` (`self.RadialForce`))
          (`/Engine/EditorBlueprintResources/ActorMacros.Switch Has Authority`
            (:`Authority`
              (bind _result (`/Engine/EditorBlueprintResources/StandardMacros.DecrementInt` (`self.Health`))
                (:`  `
                  _)))
            (:`Remote`
              _))
          (if (<= _result 0)
            (`GameplayStatics.SpawnEmitterAtLocation` "/Game/Particles/P_Explosion.P_Explosion" (`self.K2_GetActorLocation`))
            (`GameplayStatics.PlaySoundAtLocation` "/Game/Sounds/SFX/Monster_Explode.Monster_Explode" (`self.K2_GetActorLocation`))
            (`self.K2_DestroyActor`)
            (else
              (bind (_direction _newtrack_0) (`Timeline|FlashHealth` :!via `PlayFromStart`)
                (:`Update`
                  (if (> _newtrack_0 0.8)
                    (`PrimitiveComponent.SetMaterial` _skeletalmesh 0 "/Game/Models/EyeEnemy/Pupil.Pupil")
                    (else
                      (`PrimitiveComponent.SetMaterial` _skeletalmesh 0 "/Game/Models/EyeEnemy/EyeBlack.EyeBlack"))))
                (:`Event`
                  (goto _label :!via `Reset`)))))))
      (else
        (`/Engine/EditorBlueprintResources/StandardMacros.DoOnce` false :!label _label_2
          (:`Completed`
            ;[1 1 1] Hit player
            (`RadialForceComponent.FireImpulse` (`self.RadialForce`))
            (`/Game/Characters/Player1.EventReduceHealth` _asplayer_1 (`self.DamageDealt`) 350.0)
            (`GameplayStatics.PlaySoundAtLocation` "/Game/Sounds/JordansSFX/PlayerImpact.PlayerImpact" (`self.K2_GetActorLocation`))
            (`KismetSystemLibrary.Delay` 0.25)
            (goto _label_2 :!via `Reset`)))))))

(fn `UserConstructionScript`)