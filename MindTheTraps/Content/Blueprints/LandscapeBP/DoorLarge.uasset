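; DoorLarge is a large door Blueprint that opens by sinking its mesh straight down and closes by raising it back.
; BeginPlay stores the mesh's starting world location, which OpenGate and CloseGate use as the reference for their targets.
; Timelines serve as per-frame drivers for constant-speed vector interpolation of the mesh.
; Each event fires only once through an unreset DoOnce, and closing requires the Opened flag set during opening.
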(event `self.ReceiveBeginPlay`
  (set `self.OriginPos` (`SceneComponent.K2_GetComponentLocation` (`self.StaticMesh1`))))

(event `OpenGate`
  (`/Engine/EditorBlueprintResources/StandardMacros.DoOnce` false
    (:`Completed`
      (`Timeline|Open Door`
        (:`Update`
          (`SceneComponent.K2_SetWorldLocation` (`self.StaticMesh1`) (`KismetMathLibrary.VInterpTo_Constant` (`SceneComponent.K2_GetComponentLocation` (`self.StaticMesh1`)) (+ (`self.OriginPos`) (0.0 0.0 -600.0)) (`GameplayStatics.GetWorldDeltaSeconds`) 120.0) false false)
          (set `self.Opened` true))))))

(event `CloseGate`
  (if (`self.Opened`)
    (`/Engine/EditorBlueprintResources/StandardMacros.DoOnce` false
      (:`Completed`
        (`Timeline|Close Door`
          (:`Update`
            (`SceneComponent.K2_SetWorldLocation` (`self.StaticMesh1`) (`KismetMathLibrary.VInterpTo_Constant` (`SceneComponent.K2_GetComponentLocation` (`self.StaticMesh1`)) (`self.OriginPos`) (`GameplayStatics.GetWorldDeltaSeconds`) 120.0) false false)))))))

(fn `UserConstructionScript`)