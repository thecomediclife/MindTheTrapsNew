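; Large exit door that sinks 600 units when OpenDoorEvent is called and rises shut once all players reach its close volume.
; CloseVolume counts overlapping actors tagged Player and triggers closing when the count equals NumberOfPlayers and the door has opened.
; Timelines only supply update ticks for constant-speed interpolation of the mesh between its BeginPlay position and the lowered one.
; DoOnce gates make opening and closing each one-shot.
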(event `self.ReceiveBeginPlay`
  (set `self.OriginPos` (`SceneComponent.K2_GetComponentLocation` (`self.StaticMesh1`))))

(event `OpenDoorEvent`
  (`/Engine/EditorBlueprintResources/StandardMacros.DoOnce` false
    (:`Completed`
      (`Timeline|Open Door`
        (:`Update`
          (`SceneComponent.K2_SetWorldLocation` (`self.StaticMesh1`) (`KismetMathLibrary.VInterpTo_Constant` (`SceneComponent.K2_GetComponentLocation` (`self.StaticMesh1`)) (+ (`self.OriginPos`) (0.0 0.0 -600.0)) (`GameplayStatics.GetWorldDeltaSeconds`) 120.0) false false)
          (set `self.Opened` true))))))

(event `self.CloseVolume.OnComponentBeginOverlap`
  (params (OtherActor :type "Actor Object Reference") (OtherComp :type "PrimitiveComponent Object Reference") (OtherBodyIndex :type Integer) (bFromSweep :type Boolean) (SweepResult :type "HitResult Structure (by ref)"))
  (if (`self.ActorHasTag` OtherActor "Player")
    (`/Engine/EditorBlueprintResources/StandardMacros.IncrementInt` (`self.ClosePlayerCounter`)
      (:`  `
        (if (== (`self.ClosePlayerCounter`) (`self.NumberOfPlayers`))
          (if (`self.Opened`)
            (`/Engine/EditorBlueprintResources/StandardMacros.DoOnce` false
              (:`Completed`
                (`Timeline|Close Door`
                  (:`Update`
                    (`SceneComponent.K2_SetWorldLocation` (`self.StaticMesh1`) (`KismetMathLibrary.VInterpTo_Constant` (`SceneComponent.K2_GetComponentLocation` (`self.StaticMesh1`)) (`self.OriginPos`) (`GameplayStatics.GetWorldDeltaSeconds`) 120.0) false false)))))))))))

(event `self.CloseVolume.OnComponentEndOverlap`
  (params (OtherActor :type "Actor Object Reference") (OtherComp :type "PrimitiveComponent Object Reference") (OtherBodyIndex :type Integer))
  (if (`self.ActorHasTag` OtherActor "Player")
    (`/Engine/EditorBlueprintResources/StandardMacros.DecrementInt` (`self.ClosePlayerCounter`))))

(fn `UserConstructionScript`)