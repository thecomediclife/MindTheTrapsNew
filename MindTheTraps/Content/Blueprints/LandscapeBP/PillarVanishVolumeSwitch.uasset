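; Volume switch that permanently sinks a pillar mesh once the required number of players stand inside it together.
; OpenVolume overlaps count Player-tagged actors, and matching NumberOfPlayers fires a one-shot timeline.
; The timeline serves as an update driver, easing StaticMesh1 far below its BeginPlay position with VInterpTo and setting Opened.
; Players leaving only lower the count; nothing raises the mesh again.
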(event `self.ReceiveBeginPlay`
  (set `self.OriginPos` (`SceneComponent.K2_GetComponentLocation` (`self.StaticMesh1`))))

(event `self.OpenVolume.OnComponentBeginOverlap`
  (params (OtherActor :type "Actor Object Reference") (OtherComp :type "PrimitiveComponent Object Reference") (OtherBodyIndex :type Integer) (bFromSweep :type Boolean) (SweepResult :type "HitResult Structure (by ref)"))
  (if (`self.ActorHasTag` OtherActor "Player")
    (`/Engine/EditorBlueprintResources/StandardMacros.IncrementInt` (`self.OpenPlayerCounter`)
      (:`  `
        (if (== (`self.OpenPlayerCounter`) (`self.NumberOfPlayers`))
          (`/Engine/EditorBlueprintResources/StandardMacros.DoOnce` false
            (:`Completed`
              (`Timeline|Timeline_0`
                (:`Update`
                  (`SceneComponent.K2_SetWorldLocation` (`self.StaticMesh1`) (`KismetMathLibrary.VInterpTo` (`SceneComponent.K2_GetComponentLocation` (`self.StaticMesh1`)) (+ (`self.OriginPos`) (0.0 0.0 -3000.0)) (`GameplayStatics.GetWorldDeltaSeconds`) 2.0) false false)
                  (set `self.Opened` true))))))))))

(event `self.OpenVolume.OnComponentEndOverlap`
  (params (OtherActor :type "Actor Object Reference") (OtherComp :type "PrimitiveComponent Object Reference") (OtherBodyIndex :type Integer))
  (if (`self.ActorHasTag` OtherActor "Player")
    (`/Engine/EditorBlueprintResources/StandardMacros.DecrementInt` (`self.OpenPlayerCounter`))))

(fn `UserConstructionScript`)