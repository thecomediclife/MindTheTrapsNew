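; Co-op entrance door that opens once every active floor button is held by a player, with up to four buttons scaled to NumberOfPlayers.
; BeginPlay hides and disables surplus buttons; per-button overlap counters drive pressed flags and materials.
; When all required flags are set, a one-time timeline lowers the mesh by constant interpolation.
; After opening, it rises back once all players are inside CloseVolume.
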(event `self.ReceiveBeginPlay`
  (set `self.OriginPos` (`SceneComponent.K2_GetComponentLocation` (`self.StaticMesh1`)))
  (if (< (`self.NumberOfPlayers`) 4)
    (`SceneComponent.ToggleVisibility` (`self.Button4`) false)
    (`PrimitiveComponent.SetCollisionEnabled` (`self.Button4Trigger`) "NoCollision")
    (if (< (`self.NumberOfPlayers`) 3)
      (`SceneComponent.ToggleVisibility` (`self.Button3`) false)
      (`PrimitiveComponent.SetCollisionEnabled` (`self.Button3Trigger`) "NoCollision")
      (if (< (`self.NumberOfPlayers`) 2)
        (`SceneComponent.ToggleVisibility` (`self.Button2`) false)
        (`PrimitiveComponent.SetCollisionEnabled` (`self.Button2Trigger`) "NoCollision")))))

(event `self.CloseVolume.OnComponentBeginOverlap`
  (params (OtherActor :type "Actor Object Reference") (OtherComp :type "PrimitiveComponent Object Reference") (OtherBodyIndex :type Integer) (bFromSweep :type Boolean) (SweepResult :type "HitResult Structure (by ref)"))
  ;[1 1 1] Close Gate
  (if (`self.ActorHasTag` OtherActor "Player")
    (`/Engine/EditorBlueprintResources/StandardMacros.IncrementInt` (`self.ClosePlayerCounter`)
      (:`  `
        (if (== (`self.ClosePlayerCounter`) (`self.NumberOfPlayers`))
          (if (`self.Opened`)
            (`/Engine/EditorBlueprintResources/StandardMacros.DoOnce` false
              (:`Completed`
                (`Timeline|Close Door`
                  (:`Update`
                    (`SceneComponent.K2_SetWorldLocation` (`self.StaticMesh1`) (`KismetMathLibrary.VInterpTo_Constant` (`SceneComponent.K2_GetComponentLocation` (`self.StaticMesh1`)) (`self.OriginPos`) (`GameplayStatics.GetWorldDeltaSeconds`) 120.0) false false)))))))))))

(event `self.CloseVolume.OnComponentEndOverlap`
  (params (OtherActor :type "Actor Object Reference") (OtherComp :type "PrimitiveComponent Object Reference") (OtherBodyIndex :type Integer))
  ;[1 1 1] Close Gate
  (if (`self.ActorHasTag` OtherActor "Player")
    (`/Engine/EditorBlueprintResources/StandardMacros.DecrementInt` (`self.ClosePlayerCounter`))))

(event `self.Button1Trigger.OnComponentBeginOverlap`
  (params (OtherActor :type "Actor Object Reference") (OtherComp :type "PrimitiveComponent Object Reference") (OtherBodyIndex :type Integer) (bFromSweep :type Boolean) (SweepResult :type "HitResult Structure (by ref)"))
  (bind _1press (`self.1Press`))
  (bind _2press (`self.2Press`))
  (bind _3press (`self.3Press`))
  ;[1 1 1] Open Door
  (if (`self.ActorHasTag` OtherActor "Player")
    (`/Engine/EditorBlueprintResources/StandardMacros.IncrementInt` (`self.Button1Counter`)
      (:`  `
        (set `self.1Press` true)
        (`PrimitiveComponent.SetMaterial` (`self.Button1`) 0 "/Game/Materials/ButtonActivated.ButtonActivated")
        (if (== (`self.NumberOfPlayers`) 4) :!label _label
          (if (and _1press _2press _3press (`self.4Press`))
            (set `self.Pressed` true)
            (`/Engine/EditorBlueprintResources/StandardMacros.DoOnce` false :!label _label_2
              (:`Completed`
                (`Timeline|Open Door`
                  (:`Update`
                    (`SceneComponent.K2_SetWorldLocation` (`self.StaticMesh1`) (`KismetMathLibrary.VInterpTo_Constant` (`SceneComponent.K2_GetComponentLocation` (`self.StaticMesh1`)) (+ (`self.OriginPos`) (0.0 0.0 -600.0)) (`GameplayStatics.GetWorldDeltaSeconds`) 120.0) false false)
                    (set `self.Opened` true))))))
          (elif (== (`self.NumberOfPlayers`) 3)
            (if (and _1press _2press _3press)
              (set `self.Pressed` true)
              (goto _label_2))
            (elif (== (`self.NumberOfPlayers`) 2)
              (if (and _1press _2press)
                (set `self.Pressed` true)
                (goto _label_2))
              (elif (== (`self.NumberOfPlayers`) 1)
                (if _1press
                  (set `self.Pressed` true)
                  (goto _label_2))))))))))

(event `self.Button1Trigger.OnComponentEndOverlap`
  (params (OtherActor :type "Actor Object Reference") (OtherComp :type "PrimitiveComponent Object Reference") (OtherBodyIndex :type Integer))
  (bind _button1counter (`self.Button1Counter`))
  ;[1 1 1] Open Door
  (if (`self.ActorHasTag` OtherActor "Player")
    (`/Engine/EditorBlueprintResources/StandardMacros.DecrementInt` _button1counter
      (:`  `
        (if (== _button1counter 0)
          (set `self.1Press` false)
          (`PrimitiveComponent.SetMaterial` (`self.Button1`) 0 "/Game/Materials/ButtonDeactivated.ButtonDeactivated")
          (set `self.Pressed` false :!label _label_3))))))

(event `self.Button2Trigger.OnComponentBeginOverlap`
  (params (OtherActor :type "Actor Object Reference") (OtherComp :type "PrimitiveComponent Object Reference") (OtherBodyIndex :type Integer) (bFromSweep :type Boolean) (SweepResult :type "HitResult Structure (by ref)"))
  ;[1 1 1] Open Door
  (if (`self.ActorHasTag` OtherActor "Player")
    (`/Engine/EditorBlueprintResources/StandardMacros.IncrementInt` (`self.Button2Counter`)
      (:`  `
        (set `self.2Press` true)
        (`PrimitiveComponent.SetMaterial` (`self.Button2`) 0 "/Game/Materials/ButtonActivated.ButtonActivated")
        (goto _label)))))

(event `self.Button2Trigger.OnComponentEndOverlap`
  (params (OtherActor :type "Actor Object Reference") (OtherComp :type "PrimitiveComponent Object Reference") (OtherBodyIndex :type Integer))
  (bind _button2counter (`self.Button2Counter`))
  ;[1 1 1] Open Door
  (if (`self.ActorHasTag` OtherActor "Player")
    (`/Engine/EditorBlueprintResources/StandardMacros.DecrementInt` _button2counter
      (:`  `
        (if (== _button2counter 0)
          (set `self.2Press` false)
          (`PrimitiveComponent.SetMaterial` (`self.Button2`) 0 "/Game/Materials/ButtonDeactivated.ButtonDeactivated")
          (goto _label_3))))))

(event `self.Button3Trigger.OnComponentBeginOverlap`
  (params (OtherActor :type "Actor Object Reference") (OtherComp :type "PrimitiveComponent Object Reference") (OtherBodyIndex :type Integer) (bFromSweep :type Boolean) (SweepResult :type "HitResult Structure (by ref)"))
  ;[1 1 1] Open Door
  (if (`self.ActorHasTag` OtherActor "Player")
    (`/Engine/EditorBlueprintResources/StandardMacros.IncrementInt` (`self.Button3Counter`)
      (:`  `
        (set `self.3Press` true)
        (`PrimitiveComponent.SetMaterial` (`self.Button3`) 0 "/Game/Materials/ButtonActivated.ButtonActivated")
        (goto _label)))))

(event `self.Button3Trigger.OnComponentEndOverlap`
  (params (OtherActor :type "Actor Object Reference") (OtherComp :type "PrimitiveComponent Object Reference") (OtherBodyIndex :type Integer))
  (bind _button3counter (`self.Button3Counter`))
  ;[1 1 1] Open Door
  (if (`self.ActorHasTag` OtherActor "Player")
    (`/Engine/EditorBlueprintResources/StandardMacros.DecrementInt` _button3counter
      (:`  `
        (if (== _button3counter 0)
          (set `self.3Press` false)
          (`PrimitiveComponent.SetMaterial` (`self.Button3`) 0 "/Game/Materials/ButtonDeactivated.ButtonDeactivated")
          (goto _label_3))))))

(event `self.Button4Trigger.OnComponentBeginOverlap`
  (params (OtherActor :type "Actor Object Reference") (OtherComp :type "PrimitiveComponent Object Reference") (OtherBodyIndex :type Integer) (bFromSweep :type Boolean) (SweepResult :type "HitResult Structure (by ref)"))
  ;[1 1 1] Open Door
  (if (`self.ActorHasTag` OtherActor "Player")
    (`/Engine/EditorBlueprintResources/StandardMacros.IncrementInt` (`self.Button4Coutner`)
      (:`  `
        (set `self.4Press` true)
        (`PrimitiveComponent.SetMaterial` (`self.Button4`) 0 "/Game/Materials/ButtonActivated.ButtonActivated")
        (goto _label)))))

(event `self.Button4Trigger.OnComponentEndOverlap`
  (params (OtherActor :type "Actor Object Reference") (OtherComp :type "PrimitiveComponent Object Reference") (OtherBodyIndex :type Integer))
  (bind _button4coutner (`self.Button4Coutner`))
  ;[1 1 1] Open Door
  (if (`self.ActorHasTag` OtherActor "Player")
    (`/Engine/EditorBlueprintResources/StandardMacros.DecrementInt` _button4coutner
      (:`  `
        (if (== _button4coutner 0)
          (set `self.4Press` false)
          (`PrimitiveComponent.SetMaterial` (`self.Button4`) 0 "/Game/Materials/ButtonDeactivated.ButtonDeactivated")
          (goto _label_3))))))

(fn `UserConstructionScript`)