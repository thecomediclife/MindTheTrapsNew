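; EntranceVolume is a one-shot trigger volume that notifies the camera controllers when a player reaches it.
; On the server, the first Box overlap by an actor tagged Player calls SetCurrentActor, which latches an Activated flag.
; It resolves the actor it is attached to through its root component's attach parent and passes it to FindNextExit on every CamController in the world.
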(event `SetCurrentActor`
  (bind _defaultsceneroot (`self.DefaultSceneRoot`))
  (bind _returnvalue (`SceneComponent.GetAttachParent` _defaultsceneroot))
  (set `self.Activated` true)
  (if (and (`KismetSystemLibrary.IsValid` _defaultsceneroot) (`KismetSystemLibrary.IsValid` _returnvalue))
    (bind _outactors (`GameplayStatics.GetAllActorsOfClass` "/Game/Characters/CamController.CamController_C"))
    (for _array_element _outactors
      (`/Game/Characters/CamController.FindNextExit` _array_element (`ActorComponent.GetOwner` _returnvalue)))))

(event `self.Box.OnComponentBeginOverlap`
  (params (OtherActor :type "Actor Object Reference") (OtherComp :type "PrimitiveComponent Object Reference") (OtherBodyIndex :type Integer) (bFromSweep :type Boolean) (SweepResult :type "HitResult Structure (by ref)"))
  (`/Engine/EditorBlueprintResources/ActorMacros.Switch Has Authority`
    (:`Authority`
      (if (and (`self.ActorHasTag` OtherActor "Player") (not (`self.Activated`)))
        (`self.SetCurrentActor`)))))

(fn `UserConstructionScript`)