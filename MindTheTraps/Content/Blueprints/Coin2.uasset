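; Coin2 is a coin pickup that a player collects by touching its trigger sphere.
; On overlap with an actor tagged Player, it casts to Player1 and adds its Value to that player's Coins on the authority side only.
; Every machine that handles the overlap then plays the pickup sound at the coin's location and destroys the coin.
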(event `self.SphereTrigger.OnComponentBeginOverlap`
  (params (OtherActor :type "Actor Object Reference") (OtherComp :type "PrimitiveComponent Object Reference") (OtherBodyIndex :type Integer) (bFromSweep :type Boolean) (SweepResult :type "HitResult Structure (by ref)"))
  (if (`self.ActorHasTag` OtherActor "Player")
    (bind _asplayer_1 (cast `/Game/Characters/Player1` OtherActor))
    (`/Engine/EditorBlueprintResources/ActorMacros.Switch Has Authority`
      (:`Authority`
        (set `/Game/Characters/Player1.Coins` (+ (`/Game/Characters/Player1.Coins` _asplayer_1) (`self.Value`)) _asplayer_1))
      (:`Remote`
        _))
    (`GameplayStatics.PlaySoundAtLocation` "/Game/Sounds/JordansSFX/CoinGet.CoinGet" (`self.K2_GetActorLocation`) (struct) 1.0)
    (`self.K2_DestroyActor`)))

(fn `UserConstructionScript`)