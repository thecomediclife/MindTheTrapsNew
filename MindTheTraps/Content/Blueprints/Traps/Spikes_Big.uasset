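; Big spike trap actor that hurts players entering its trigger volume.
; On server-side overlap, while Active, it fires a radial force impulse sized at BeginPlay, then damages a Player2 with a coin-eject speed and plays an impact sound.
; DeactivateAfterPlay limits activations; any overlapping actor consumes one, but the trap destroys itself at zero only after a successful Player2 hit.
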(event `self.ReceiveBeginPlay`
  (set `RadialForceComponent.Radius` (`self.RadialForceSize`) (`self.RadialForce`)))

(event `self.TriggerVolume.OnComponentBeginOverlap`
  (params (OtherActor :type "Actor Object Reference") (OtherComp :type "PrimitiveComponent Object Reference") (OtherBodyIndex :type Integer) (bFromSweep :type Boolean) (SweepResult :type "HitResult Structure (by ref)"))
  (`/Engine/EditorBlueprintResources/ActorMacros.Switch Has Authority`
    (:`Authority`
      (set `self.OverlapTarget` OtherActor)
      (if (`self.Active`)
        (if (`self.DeactivateAfterPlay`)
          (if (> (`self.NumberOfActivations`) 0)
            (bind _result (`/Engine/EditorBlueprintResources/StandardMacros.DecrementInt` (`self.NumberOfActivations`))
              (:`  `
                (set `self.NumberOfActivations` _result)
                (`RadialForceComponent.FireImpulse` (`self.RadialForce`) :!label _label)
                (bind _asplayer_2 (cast `/Game/Characters/Player2` (`self.OverlapTarget`)))
                (`/Game/Characters/Player2.EventReduceHealth` _asplayer_2 (`self.DamageDealt`) 350.0)
                (`GameplayStatics.PlaySoundAtLocation` "/Game/Sounds/JordansSFX/PlayerImpact.PlayerImpact" (`self.K2_GetActorLocation`) (struct) 1.0)
                (if (and (== (`self.NumberOfActivations`) 0) (`self.DeactivateAfterPlay`))
                  (`self.K2_DestroyActor`)))))
          (else
            (goto _label)))))))

(fn `UserConstructionScript`)