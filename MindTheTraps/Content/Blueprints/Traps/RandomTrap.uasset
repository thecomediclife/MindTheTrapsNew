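; RandomTrap is a placeable spawner actor that puts a randomly chosen trap at its location when play begins.
; BeginPlay calls SpawnRandomTrap, which picks a random entry from the TrapsList class array and spawns it if the class is valid.
; The spawned trap uses only the spawner's location, with zero rotation and unit scale, and the spawner stays in the level.
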(event `SpawnRandomTrap`
  (bind _trapslist (`self.TrapsList`))
  (bind _output_get (set `self.RandIndex` (`KismetMathLibrary.RandomIntegerInRange` 0 (- (`KismetArrayLibrary.Array_Length` _trapslist) 1))))
  (bind _item (`KismetArrayLibrary.Array_Get` _trapslist _output_get))
  (if (`KismetSystemLibrary.IsValidClass` _item)
    (`|SpawnActorFromClass` _item (`KismetMathLibrary.MakeTransform` (`self.K2_GetActorLocation`)) "Undefined" "OverrideRootScale")))

(event `self.ReceiveBeginPlay`
  (`self.SpawnRandomTrap`))

(event `self.ReceiveActorBeginOverlap`
  (params (OtherActor :type "Actor Object Reference")))

(event `self.ReceiveTick`
  (params (DeltaSeconds :type "Float (single-precision)")))

(fn `UserConstructionScript`)