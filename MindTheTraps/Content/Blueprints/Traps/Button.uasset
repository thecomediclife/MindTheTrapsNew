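; Pressure-button trap trigger that fires attached bow-and-arrow statue and ceiling spike traps when a Player-tagged actor overlaps it.
; On the server, a DoOnce-gated overlap decrements the use count, activates each attached trap and plays staggered arrow sounds.
; The button destroys itself when uses run out, otherwise re-arms.
; The spike sound branch is empty, and Spikes is only ever set false while Arrow is never reset.
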(event `self.Trigger.OnComponentBeginOverlap`
  (params (OtherActor :type "Actor Object Reference") (OtherComp :type "PrimitiveComponent Object Reference") (OtherBodyIndex :type Integer) (bFromSweep :type Boolean) (SweepResult :type "HitResult Structure (by ref)"))
  (bind _returnvalue (`self.K2_GetActorLocation`))
  (`/Engine/EditorBlueprintResources/ActorMacros.Switch Has Authority`
    (:`Authority`
      (`self.ResetBools`)
      (if (`self.ActorHasTag` OtherActor "Player")
        (`/Engine/EditorBlueprintResources/StandardMacros.DoOnce` false :!label _label
          (:`Completed`
            (`/Engine/EditorBlueprintResources/StandardMacros.DecrementInt` (`self.ActivateNumberOfTime`)
              (:`  `
                (for _array_element (`self.AttachedActors`)
                  (bind _asboobie_trap_statue_bow_and_arrow (cast `/Game/Blueprints/Traps/BoobieTrap_StatueBowAndArrow` _array_element)
                    (:`then`
                      (`/Game/Blueprints/Traps/BoobieTrap_StatueBowAndArrow.ActivateTrap` _asboobie_trap_statue_bow_and_arrow)
                      (set `self.Arrow` true))
                    (:`CastFailed`
                      (bind _asboobie_trap_ceiling_spikes (cast `/Game/Blueprints/Traps/BoobieTrap_CeilingSpikes` _array_element))
                      (`/Game/Blueprints/Traps/BoobieTrap_CeilingSpikes.ActivateTrap` _asboobie_trap_ceiling_spikes)
                      (set `self.Spikes` false))))
                (if (`self.Arrow`)
                  (`GameplayStatics.PlaySoundAtLocation` "/Game/Sounds/JordansSFX/ArrowTwang.ArrowTwang" _returnvalue)
                  (`KismetSystemLibrary.Delay` 0.07)
                  (`GameplayStatics.PlaySoundAtLocation` "/Game/Sounds/JordansSFX/ArrowSwoosh.ArrowSwoosh" _returnvalue))
                ;[1 1 1] Play Sound for Spikes
                (if (`self.Spikes`)
                  _
                  (else
                    _))
                (if (<= (`self.ActivateNumberOfTime`) 0)
                  (`/Engine/EditorBlueprintResources/ActorMacros.Switch Has Authority`
                    (:`Authority`
                      (`self.K2_DestroyActor`)))
                  (else
                    (goto _label :!via `Reset`)))))))))))

(fn `ResetBools`
  (set `self.Spikes` false)
  (set `self.Spikes` false))

(fn `UserConstructionScript`)