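; Arrow projectile actor, filed with the traps, that reacts to striking players and cleans itself up.
; On the server, a timeline starts at BeginPlay and destroys the arrow when it finishes.
; Overlapping an actor tagged Player plays arrow and player impact sounds locally, then destroys the arrow on authority only.
; The Blueprint applies no damage, and its component hit event is empty.
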(event `self.ReceiveBeginPlay`
  (`/Engine/EditorBlueprintResources/ActorMacros.Switch Has Authority`
    (:`Authority`
      (`Timeline|Selfdesstruct`
        (:`Finished`
          (`self.K2_DestroyActor`))))))

(event `self.Collision.OnComponentBeginOverlap`
  (params (OtherActor :type "Actor Object Reference") (OtherComp :type "PrimitiveComponent Object Reference") (OtherBodyIndex :type Integer) (bFromSweep :type Boolean) (SweepResult :type "HitResult Structure (by ref)"))
  (bind _returnvalue (`self.K2_GetActorLocation`))
  (if (`self.ActorHasTag` OtherActor "Player")
    (`GameplayStatics.PlaySoundAtLocation` "/Game/Sounds/JordansSFX/Arrow_Impact.Arrow_Impact" _returnvalue)
    (`GameplayStatics.PlaySoundAtLocation` "/Game/Sounds/JordansSFX/PlayerImpact.PlayerImpact" _returnvalue)
    (`/Engine/EditorBlueprintResources/ActorMacros.Switch Has Authority`
      (:`Authority`
        (`self.K2_DestroyActor`)))))

(event `self.Collision.OnComponentHit`
  (params (OtherActor :type "Actor Object Reference") (OtherComp :type "PrimitiveComponent Object Reference") (NormalImpulse :type "Vector Structure") (Hit :type "HitResult Structure (by ref)")))

(fn `UserConstructionScript`)